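; BP_Projectile is an enemy projectile that damages the player or can be deflected by the player's sword, self-destroying after a short lifetime.
; On sphere overlap with a player-held BP_Sword, it zeroes the ProjectileMovement speed settings and applies a velocity-change impulse.
; That impulse mirrors its velocity about the player's forward vector, scaled by ReflectSpeed.
; Overlapping BP_Player directly calls RecievedDamage without destroying the projectile.
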(event `self.ReceiveBeginPlay`
  (`KismetSystemLibrary.Delay` 3.0)
  (`self.K2_DestroyActor`))

(event `self.SphereCollision.OnComponentBeginOverlap`
  (params (OverlappedComponent :type "PrimitiveComponent Object Reference") (OtherActor :type "Actor Object Reference") (OtherComp :type "PrimitiveComponent Object Reference") (OtherBodyIndex :type Integer) (bFromSweep :type Boolean) (SweepResult :type "HitResult Structure (by ref)"))
  (bind _projectilemovement (`self.ProjectileMovement`))
  (bind _returnvalue (`self.GetVelocity` self))
  (`|ExecutionSequence`
    (:`then_0`
      ; 칼로 튕겨냈을 때
      (bind _asbp_sword (cast `/Game/LHM/Blueprints/Player/BP_Sword` OtherActor))
      (bind _asbp_player (cast `/Game/LHM/Blueprints/Player/BP_Player` (`self.GetAttachParentActor` _asbp_sword)))
      (set `ProjectileMovementComponent.InitialSpeed` 0.0 _projectilemovement)
      (set `ProjectileMovementComponent.MaxSpeed` 0.0 _projectilemovement)
      (bind _returnvalue_2 (`self.GetActorForwardVector` _asbp_player))
      (`PrimitiveComponent.AddImpulse` (`self.SphereCollision`) (* (- _returnvalue (* (* (`KismetMathLibrary.Dot_VectorVector` _returnvalue _returnvalue_2) 2.0) _returnvalue_2)) (`self.ReflectSpeed`)) "None" true)
      (`KismetSystemLibrary.PrintString` "Successed Reflect"))
    (:`then_1`
      ; 플레이어가 총알에 맞았을 때
      (bind _asbp_player_2 (cast `/Game/LHM/Blueprints/Player/BP_Player` OtherActor))
      (`/Game/LHM/Blueprints/Player/BP_Player.Recieved Damage` _asbp_player_2 10.0))))

(fn `UserConstructionScript`)