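; BP_Enemy is a rifle enemy that switches between Patrol, Attack and Dead states, dispatched on Tick and mirrored to its AI Blackboard.
; Pawn sensing sets the player as target and starts Attack; rescanning living players returns it to Patrol beyond sight radius.
; Attack plays a delayed fire montage, spawning projectiles from the muzzle toward the target.
; Damage sets Dead when remaining HP is zero or above (apparently inverted), destroying the actor.
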(event `self.ReceiveTick`
  (params (DeltaSeconds :type "Float (single-precision)"))
  ; 실시간으로 상태를 체크하고 상태에 따른 행동 함수 호출
  (switch `/Game/LHM/Blueprints/Enemy/E_EnemyState` (`self.State`)
    (:`NewEnumerator0`
      (`self.On Patrol`))
    (:`NewEnumerator2`
      (`self.On Attack`))
    (:`NewEnumerator3`
      (`self.On Dead`))))

(event `On Patrol`
  ; 상태에 따른 행동 이벤트
)

(event `On Attack`
  ; 상태에 따른 행동 이벤트
  (`/Engine/EditorBlueprintResources/StandardMacros.IsValid` (`self.Instigator`)
    (:`Is Valid`
      (bind _asbp_player (cast `/Game/LHM/Blueprints/Player/BP_Player` (`self.Instigator`)))
      (bind _result (`/Game/LHM/Blueprints/Player/BP_Player.Is Player Dead` _asbp_player))
      (if _result
        (`self.Detect Player`)
        (else
          (`KismetSystemLibrary.Delay` 2.0)
          (`|PlayMontage` (`self.Mesh`) "/Game/Enemy/Animations/Montages/AM_Rifle_Fire_Aim.AM_Rifle_Fire_Aim" 1.0 0.0 "Fire"
            (:`then`
              (`self.Shoot up`)
              (`self.Detect Player`))))))
    (:`Is Not Valid`
      (`self.Detect Player`))))

(event `On Dead`
  ; 상태에 따른 행동 이벤트
  (`self.Die`))

(event `self.ReceiveAnyDamage`
  (params (Damage :type "Float (single-precision)") (DamageType :type "DamageType Object Reference") (InstigatedBy :type "Controller Object Reference") (DamageCauser :type "Actor Object Reference"))
  ; 데미지 처리
  (bind _output_get (set `self.HP` (- (`self.HP`) Damage)))
  (if (>= _output_get 0.0)
    (`self.Set State` "NewEnumerator3")))

(event `self.PawnSensing.OnSeePawn`
  (params (Pawn :type "Pawn Object Reference"))
  ; 플레이어 감지
  (if (`|EnumEquality` (`self.State`) "NewEnumerator0")
    (cast `/Game/LHM/Blueprints/Player/BP_Player` Pawn)
    (`self.Set State` "NewEnumerator2")
    (bind _output_get (set `self.Instigator` Pawn))
    (`BlackboardComponent.SetValueAsObject` (`AIController.Blackboard` (`AIBlueprintHelperLibrary.GetAIController` self)) (`self.Target Player Key`) _output_get)))

(event `Set State`
  (params (`New State` :type "/Game/LHM/Blueprints/Enemy/E_EnemyState Enum" :default "NewEnumerator0"))
  ; 상태 변경 이벤트
  (if (`|EnumInequality` (`self.State`) "NewEnumerator3")
    (if (`|EnumInequality` (`self.State`) `New State`)
      (bind _output_get (set `self.State` `New State`))
      (`BlackboardComponent.SetValueAsEnum` (`AIBlueprintHelperLibrary.GetBlackboard` (`AIBlueprintHelperLibrary.GetAIController` self)) (`self.State Key`) _output_get))))

(fn `Detect Player`
  (bind _instigator (`self.Instigator`))
  (bind _outactors (`GameplayStatics.GetAllActorsOfClass` "/Game/LHM/Blueprints/Player/BP_Player.BP_Player_C"))
  (for _array_element _outactors
    (bind _result (`/Game/LHM/Blueprints/Player/BP_Player.Is Player Dead` _array_element))
    (if (not _result)
      (bind _output_get (set `self.Instigator` _array_element))
      (`BlackboardComponent.SetValueAsObject` (`AIController.Blackboard` (`AIBlueprintHelperLibrary.GetAIController` self)) (`self.Target Player Key`) _output_get)
      (`/Engine/EditorBlueprintResources/StandardMacros.IsValid` _instigator
        (:`Is Valid`
          (if (> (`KismetMathLibrary.Vector_Distance` (`self.K2_GetActorLocation` _instigator) (`self.K2_GetActorLocation`)) (`PawnSensingComponent.SightRadius` (`self.PawnSensing`)))
            (`self.Set State` "NewEnumerator0")))))))

(fn `Die`
  (`self.Set State` "NewEnumerator3")
  (`self.K2_DestroyActor`))

(fn `Shoot up`
  (bind _returnvalue (`SceneComponent.GetSocketLocation` (`self.Mesh`) "Muzzle"))
  (bind (_returnvalue_x _returnvalue_y _returnvalue_z) (`KismetMathLibrary.BreakVector` (`self.K2_GetActorLocation` (`self.Instigator`))))
  (`|SpawnActorFromClass` "/Game/LHM/Blueprints/Enemy/BP_Projectile.BP_Projectile_C" (`KismetMathLibrary.MakeTransform` _returnvalue (`KismetMathLibrary.FindLookAtRotation` _returnvalue (`KismetMathLibrary.MakeVector` _returnvalue_x _returnvalue_y (+ _returnvalue_z 75.0)))) "Undefined" "MultiplyWithRoot" null null))

(fn `UserConstructionScript`)