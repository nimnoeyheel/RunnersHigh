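; BP_Sword is the player's melee weapon actor, which damages whatever its hit box overlaps during an attack.
; The box collision starts disabled, switches to query-only on OnAttackStart and turns off again on OnAttackEnd.
; Each overlap applies fixed damage to the other actor, crediting player controller 0 as instigator and the sword as causer.
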(event `self.ReceiveBeginPlay`
  (`PrimitiveComponent.SetCollisionEnabled` (`self.BoxCollision`) "NoCollision"))

(event `self.BoxCollision.OnComponentBeginOverlap`
  (params (OverlappedComponent :type "PrimitiveComponent Object Reference") (OtherActor :type "Actor Object Reference") (OtherComp :type "PrimitiveComponent Object Reference") (OtherBodyIndex :type Integer) (bFromSweep :type Boolean) (SweepResult :type "HitResult Structure (by ref)"))
  (`GameplayStatics.ApplyDamage` OtherActor 10.0 (`GameplayStatics.GetPlayerController` 0) self))

(event `On Attack Start`
  (`PrimitiveComponent.SetCollisionEnabled` (`self.BoxCollision`) "QueryOnly"))

(event `On Attack End`
  (`PrimitiveComponent.SetCollisionEnabled` (`self.BoxCollision`) "NoCollision"))

(fn `UserConstructionScript`)